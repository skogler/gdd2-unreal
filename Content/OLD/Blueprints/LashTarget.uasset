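; LashTarget is a clickable physics actor that the player lashes with mouse drags to apply persistent directional forces, highlighting its mesh on hover.
; Click and release positions are subtracted in screen space, mapped onto world Y/Z, and appended to an array of lash vectors.
; Tick applies every vector as a force scaled by mass and delta time, decaying each per frame without ever removing it.
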(event OnBeginCursorOver(StaticMesh)
  (params (TouchedComponent :type Primitive%20Component%20Object%20Reference))
  ;[1 1 1] Mouseover highlight
  (Rendering|Material|SetMaterial 0 "/Game/OLD/Blueprints/LashingMaterial.LashingMaterial"))

(event OnEndCursorOver(StaticMesh)
  (params (TouchedComponent :type Primitive%20Component%20Object%20Reference))
  ;[1 1 1] Mouseover highlight
  (Rendering|Material|SetMaterial 0 "/Game/OLD/Meshes/CubeMaterial.CubeMaterial"))

(event EventTick
  (params (DeltaSeconds :type Float%20%28single-precision%29))
  (bind _directionallashes (Variables|Default|GetdirectionalLashes))
  ;[1 1 1] apply forces from array each tick
  (for (_array_element _array_index) _directionallashes
    (Physics|AddForce (* _array_element (* DeltaSeconds (* (Physics|GetMass) 5e+02))) "None" false)
    ;[1 1 1] dampening
    (Utilities|Array|SetArrayElem _directionallashes _array_index (* _array_element 0.99))))

(event MouseInput|EventActorOnClicked
  (bind _returnvalue (Game|GetPlayerController 0))
  (bind (_locationx _locationy) (Game|Player|GetMousePosition _returnvalue))
  ;[1 1 1] add force to array on mouse drag
  (Utilities|FlowControl|Sequence
    (:then_0
      (Variables|Default|Setdragging true)
      (Variables|Default|SetdragStart (Math|Vector|MakeVector 0.0 _locationx _locationy)))))

(event Input|MouseEvents|LeftMouseButton
  (bind _returnvalue (Game|GetPlayerController 0))
  (bind (_locationx _locationy) (Game|Player|GetMousePosition _returnvalue))
  ;[1 1 1] add force to array on mouse drag
  (:Released
    (if (Variables|Default|Getdragging)
      (Variables|Default|Setdragging false)
      (Utilities|Array|Add (Variables|Default|GetdirectionalLashes) (- (Variables|Default|GetdragStart) (Math|Vector|MakeVector 0.0 _locationx _locationy))))))

(fn ConstructionScript)