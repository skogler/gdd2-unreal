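; BP_Player is the player Blueprint for a shooter with asteroids, handling weapons, collision damage and game over.
; Space spawns unlimited laser shots and Left Ctrl spawns ammo-limited rockets along the control rotation, both sharing fire sound and camera shake.
; Hitting an asteroid applies huge radial damage, spawns a scaled-up explosion and decrements Health, calling game over at zero.
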(event EventHit
  (params (MyComp :type Primitive%20Component%20Object%20Reference) (Other :type Actor%20Object%20Reference) (OtherComp :type Primitive%20Component%20Object%20Reference) (bSelfMoved :type Boolean) (HitLocation :type Vector :default "0, 0, 0") (HitNormal :type Vector :default "0, 0, 0") (NormalImpulse :type Vector :default "0, 0, 0") (Hit :type Hit%20Result%20Structure%20%28by%20ref%29))
  (Utilities|Casting|CastToBP_Asteroid Other)
  (Game|Damage|ApplyRadialDamage 1e+04 HitLocation 1e+05 "/Engine/EngineDamageTypes/DmgTypeBP_Environmental.DmgTypeBP_Environmental_C" 0 self 0 true "ECC_Visibility")
  (bind _returnvalue (Effects|SpawnEmitteratLocation "/Game/Particles/P_Asteroid_Explosion.P_Asteroid_Explosion" (Transformation|GetActorLocation)))
  (Transformation|SetWorldScale3D _returnvalue "100.000000,100.000000,100.000000")
  (Variables|Default|SetHealth (- (Variables|Default|GetHealth) 1))
  (if (== (Variables|Default|GetHealth) 0)
    (Default|CallGameOver)))

(event Input|KeyboardEvents|LeftCtrl
  (bind _returnvalue (Transformation|GetActorLocation))
  (bind _returnvalue_2 (Pawn|GetControlRotation :!class /Script/Engine.Pawn))
  ;[1 1 1] Spawn Rocket
  (:Pressed
    (if (> (Variables|Default|GetAmmo) 0)
      (Variables|Default|SetAmmo (- (Variables|Default|GetAmmo) 1))
      (Game|SpawnActorfromClass "/Game/Blueprints/BP_Rocket.BP_Rocket_C" (Math|Transform|MakeTransform (+ (Transformation|GetActorLocation) (Math|Vector|RotateVector "0, 0, 0" _returnvalue_2)) _returnvalue_2) false 0)
      ;[1 1 1] Spawn PLASMA projectile
      (Audio|PlaySoundatLocation "/Game/Audio/FirstPerson_WeaponFire.FirstPerson_WeaponFire" _returnvalue) ; Play firing sound
      (Camera|PlayWorldCameraShake "/Game/Blueprints/BP_Laser_ScreenShake.BP_Laser_ScreenShake_C" _returnvalue 0.0 5e+02))))

(event Input|KeyboardEvents|SpaceBar
  (bind _returnvalue (Transformation|GetActorLocation))
  (bind _returnvalue_2 (Pawn|GetControlRotation :!class /Script/Engine.Pawn))
  ;[1 1 1] Spawn PLASMA projectile
  (:Pressed
    (Game|SpawnActorfromClass "/Game/Blueprints/BP_Lasershot.BP_Lasershot_C" (Math|Transform|MakeTransform (+ (Transformation|GetActorLocation) (Math|Vector|RotateVector "0, 0, 0" _returnvalue_2)) _returnvalue_2) false 0) ; Spawn projectile
    (Audio|PlaySoundatLocation "/Game/Audio/FirstPerson_WeaponFire.FirstPerson_WeaponFire" _returnvalue) ; Play firing sound
    (Camera|PlayWorldCameraShake "/Game/Blueprints/BP_Laser_ScreenShake.BP_Laser_ScreenShake_C" _returnvalue 0.0 5e+02)))

(fn ConstructionScript)